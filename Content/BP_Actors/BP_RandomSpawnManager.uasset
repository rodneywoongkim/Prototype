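; BP_RandomSpawnManager spawns a set number of randomly chosen actors at the level's spawn points when play begins.
; On BeginPlay it gathers every BP_SpawnPoint, optionally shuffles the list, then spawns a random class from its Class array at each point until Count runs out.
; Only each point's world location is used, and each point is used at most once, so the number of points caps the total.
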(event Custom|Break
  (Utilities|Array|ForEachLoopwithBreak (Variables|Default|GetSpawnPoints)) ; enters at Break
)

(event EventBeginPlay
  (bind _outactors (Actor|GetAllActorsOfClass "/Game/BP_Actors/BP_SpawnPoint.BP_SpawnPoint_C"))
  (bind _output_get (Variables|Default|SetSpawnPoints _outactors))
  (if (Variables|Default|GetShuffle)
    (Utilities|Array|Shuffle _output_get))
  (bind _array_element (Utilities|Array|ForEachLoopwithBreak (Variables|Default|GetSpawnPoints))
    (:LoopBody
      (if (== (Variables|Default|GetCount) 0)
        (CallFunction|Break)
        (else
          (bind _output_get_2 (Variables|Default|SetRandom%20Spawn _array_element))
          (Game|SpawnActorfromClass (.OutItem (Utilities|Array|Random (Variables|Default|GetClass))) (Math|Conversions|ToTransform(Vector) (Transformation|GetWorldLocation (Variables|/Script/Engine.Actor|GetRootComponent _output_get_2))) "Undefined" "SelectDefaultAtRuntime" 0 0)
          (Variables|Default|SetCount (- (Variables|Default|GetCount) 1)))))))

(event Collision|EventActorBeginOverlap
  (params (OtherActor :type Actor%20Object%20Reference)))

(event EventTick
  (params (DeltaSeconds :type Float%20%28single-precision%29)))

(fn ConstructionScript)