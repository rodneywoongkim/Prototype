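; BP_Volume_RandomSpawn is a placeable box volume that scatters randomly chosen actors over the surfaces beneath it at BeginPlay.
; The construction script sizes the box from VolumeScale.
; For each of Count attempts, it samples random points in the box and runs a long downward Visibility trace with debug drawing.
; A valid hit spawns a random entry from the Class array at the impact location, unrotated and at unit scale.
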(event EventBeginPlay
  (bind _box (Variables|Default|GetBox))
  (bind _returnvalue (Transformation|GetWorldLocation _box))
  (bind _returnvalue_2 (Components|Box|GetScaledBoxExtent _box))
  (bind _returnvalue_3 (Math|Random|RandomPointinBoundingBox _returnvalue _returnvalue_2))
  (bind _returnvalue_4 (Math|Transform|MakeTransform _returnvalue_3))
  (bind _location (Math|Transform|BreakTransform _returnvalue_4))
  (bind (_x _y _z) (Math|Vector|BreakVector _location))
  (for _index (range 0 (- (Variables|Default|GetCount) 1))
    (bind (_outhit _returnvalue_5) (Collision|LineTraceByChannel (Math|Vector|MakeVector _x _y (+ _z 1e+02)) (Math|Vector|MakeVector _x _y (- _z 2e+04)) "TraceTypeQuery1" false 0 "ForDuration"))
    (if _returnvalue_5
      (Utilities|IsValid (.HitActor (Collision|BreakHitResult _outhit))
        (:Is%20Valid
          (Game|SpawnActorfromClass (.OutItem (Utilities|Array|Random (Variables|Default|GetClass))) (Math|Transform|MakeTransform (.Location (Collision|BreakHitResult _outhit))) "Undefined" "SelectDefaultAtRuntime" 0 0))))))

(event Collision|EventActorBeginOverlap
  (params (OtherActor :type Actor%20Object%20Reference)))

(event EventTick
  (params (DeltaSeconds :type Float%20%28single-precision%29)))

(fn ConstructionScript
  (Transformation|SetWorldScale3D (Variables|Default|GetBox) (Variables|Default|GetVolumeScale)))