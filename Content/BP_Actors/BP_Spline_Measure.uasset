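; BP_Spline_Measure is a measuring actor that shows spline distances in meters as in-world text.
; Its construction script branches on PointLength: when true, it adds an enlarged text render above each spline point, turned to the point's rotation plus a half-turn yaw, showing cumulative distance.
; Otherwise, the existing TextRender shows the total spline length.
; The event graph has no active logic.
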(event EventBeginPlay)

(event Collision|EventActorBeginOverlap
  (params (OtherActor :type Actor%20Object%20Reference)))

(event EventTick
  (params (DeltaSeconds :type Float%20%28single-precision%29)))

(fn ConstructionScript
  (bind _spline (Variables|Default|GetSpline))
  (if (Variables|Default|GetPoint%20Length)
    (for _index (range 0 (- (Spline|GetNumberOfSplinePoints (Variables|Default|GetSpline)) 1))
      (bind _returnvalue (AddComponent|AddTextRenderComponent false (Math|Transform|MakeTransform (+ (Spline|GetLocationatSplinePoint _spline _index "Local") "0.000000,0.000000,50.000000") (Math|Rotator|MakeRotator (.roll (Spline|GetRotationatSplinePoint _spline _index "Local")) (.pitch (Spline|GetRotationatSplinePoint _spline _index "Local")) (+ (.yaw (Spline|GetRotationatSplinePoint _spline _index "Local")) 1.8e+02)) "2.000000,2.000000,2.000000")))
      (Rendering|Components|TextRender|SetText _returnvalue (Utilities|Text|FormatText "{0}m" (Utilities|Text|ToText(Float) (/ (Spline|GetDistanceAlongSplineatSplinePoint _spline _index) 1e+02) "HalfToEven"))))
    (else
      (Rendering|Components|TextRender|SetText (Variables|Default|GetTextRender) (Utilities|Text|FormatText "{0}m" (Utilities|Text|ToText(Float) (/ (Spline|GetSplineLength (Variables|Default|GetSpline)) 1e+02) "HalfToEven"))))))