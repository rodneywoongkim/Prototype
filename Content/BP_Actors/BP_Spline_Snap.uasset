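; BP_Spline_Snap is a spline actor that drops its points onto the landscape or other surfaces below.
; When SnapToLandscape is ticked, the Construction Script runs a vertical Visibility line trace, with debug drawing, through each spline point.
; Each point moves to the trace's hit location without a hit check, and the flag resets, acting as a one-shot button.
; The event graph holds only empty default events.
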(event EventBeginPlay)

(event Collision|EventActorBeginOverlap
  (params (OtherActor :type Actor%20Object%20Reference)))

(event EventTick
  (params (DeltaSeconds :type Float%20%28single-precision%29)))

(fn ConstructionScript
  (bind _spline (Variables|Default|GetSpline))
  ;[0 0 0 1 15] 랜드스케이프 스냅
  (if (Variables|Default|GetSnap%20To%20Landscape)
    (for _index (range 0 (- (Spline|GetNumberOfSplinePoints _spline) 1))
      (bind _outhit (Collision|LineTraceByChannel (Math|Vector|MakeVector (.x (Spline|GetLocationatSplinePoint _spline _index "World")) (.y (Spline|GetLocationatSplinePoint _spline _index "World")) (+ (.z (Spline|GetLocationatSplinePoint _spline _index "World")) 2e+03)) (Math|Vector|MakeVector (.x (Spline|GetLocationatSplinePoint _spline _index "World")) (.y (Spline|GetLocationatSplinePoint _spline _index "World")) (- (.z (Spline|GetLocationatSplinePoint _spline _index "World")) 2e+03)) "TraceTypeQuery1" false 0 "ForDuration"))
      (Spline|SetLocationatSplinePoint _spline _index (.location _outhit) "World" true)
      (Variables|Default|SetSnap%20To%20Landscape false))))