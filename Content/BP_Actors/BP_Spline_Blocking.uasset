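; BP_Spline_Blocking is a construction-time tool that lays collidable spline mesh segments along a spline, apparently as an adjustable-height blocking barrier.
; The construction script derives segment length from the Cube mesh's X bounds and divides the spline length by it to set the segment count.
; Each segment follows the spline with tangents clamped to segment length to limit distortion, while Height scales its Z.
; The event graph holds no logic.
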(event EventBeginPlay)

(event Collision|EventActorBeginOverlap
  (params (OtherActor :type Actor%20Object%20Reference)))

(event EventTick
  (params (DeltaSeconds :type Float%20%28single-precision%29)))

(fn ConstructionScript
  (bind _spline (Variables|Default|GetSpline))
  (bind _cube (Variables|Default|GetCube))
  (bind _spline_2 (Variables|Default|GetSpline))
  (bind _staticmesh (Variables|/Script/Engine.StaticMeshComponent|GetStaticMesh _cube))
  (bind _returnvalue (StaticMesh|GetBoundingBox _staticmesh))
  (bind _output_get (Variables|Default|SetXlength (.x (+ (Math|Vector|VectorGetAbs (.min _returnvalue)) (Math|Vector|VectorGetAbs (.max _returnvalue))))))
  (for _index (range 0 (Math|Float|Truncate (/ (Spline|GetSplineLength (Variables|Default|GetSpline)) _output_get)))
    (bind _returnvalue_2 (AddComponent|AddSplineMeshComponent false (Math|Transform|MakeTransform "0, 0, 0" "0, 0, 0" (Math|Vector|MakeVector 1.0 1.0 (Math|Conversions|ToFloat(Integer) (Variables|Default|GetHeight))))))
    (Collision|SetCollisionEnabled _returnvalue_2 "QueryAndPhysics")
    (SplineMesh|SetForwardAxis _returnvalue_2 "X" true)
    (SplineMesh|SetStartandEnd _returnvalue_2 (Spline|GetLocationatDistanceAlongSpline _spline_2 (* _index (Variables|Default|GetXlength)) "Local") (Math|Vector|ClampVectorSize (Spline|GetTangentatDistanceAlongSpline _spline_2 (* _index (Variables|Default|GetXlength)) "Local") 0.0 (Variables|Default|GetXlength)) (Spline|GetLocationatDistanceAlongSpline _spline (* (+ _index 1) (Variables|Default|GetXlength)) "Local") (Math|Vector|ClampVectorSize (Spline|GetTangentatDistanceAlongSpline _spline (* (+ _index 1) (Variables|Default|GetXlength)) "Local") 0.0 (Variables|Default|GetXlength)) true :!class /Script/Engine.SplineMeshComponent)))